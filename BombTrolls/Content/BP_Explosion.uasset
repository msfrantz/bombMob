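; BP_Explosion is a short-lived explosion actor that damages players caught in its box and removes itself two seconds after spawning.
; Its Box overlap casts Player-tagged actors to BP_Player and calls ServerTakeDamage with an Explosion damage type and the explosion's Creator.
; BeginPlay disables the box collision after a brief delay, limiting the damage window, and calls ClientSpawnExplosion to attach the Explosion particle system to the box.
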(event OnComponentBeginOverlap(Box)
  (params (OverlappedComponent :type Primitive%20Component%20Object%20Reference) (OtherActor :type Actor%20Object%20Reference) (OtherComp :type Primitive%20Component%20Object%20Reference) (OtherBodyIndex :type Integer) (bFromSweep :type Boolean) (SweepResult :type Hit%20Result%20Structure%20%28by%20ref%29))
  (Utilities|IsValid OtherActor
    (:Is%20Valid
      (if (Actor|ActorHasTag OtherActor "Player")
        (bind _asbp_player (Utilities|Casting|CastToBP_Player OtherActor))
        (Default|ServerTakeDamage _asbp_player "Explosion" (Variables|Default|GetCreator))))))

(event Custom|ClientSpawnExplosion
  (Niagara|SpawnSystemAttached "/Game/Art/Explosion.Explosion" (Variables|Default|GetBox) "None" "0, 0, 0" "0, 0, 0" "KeepRelativeOffset" true))

(event EventBeginPlay
  (Utilities|FlowControl|Sequence
    (:then_0
      (Utilities|FlowControl|Delay 2.0)
      (Actor|DestroyActor))
    (:then_1
      (Utilities|FlowControl|Delay 0.3)
      (Collision|SetCollisionEnabled (Variables|Default|GetBox) "NoCollision"))
    (:then_2
      (CallFunction|ClientSpawnExplosion))))

(event EventTick
  (params (DeltaSeconds :type Float%20%28single-precision%29)))

(fn ConstructionScript)