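; BP_Camera2 is a follow camera actor that becomes the local player's view and tracks the controlled pawn.
; One second after BeginPlay it registers itself as ClientCamera on BP_Player, stores the pawn and sets itself as the view target.
; A looping 0.001-second timer, rather than Tick, calls UpdateCamera to snap the actor to the pawn's location, leaving rotation untouched.
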(event Custom|UpdateCamera
  (Transformation|SetActorLocation (Transformation|GetActorLocation (Variables|Default|GetPawnToFollow)) false false))

(event EventTick
  (params (DeltaSeconds :type Float%20%28single-precision%29)))

(event EventBeginPlay
  (bind _returnvalue (Game|GetPlayerController 0))
  (bind _returnvalue_2 (Pawn|GetControlledPawn _returnvalue))
  (Utilities|FlowControl|Delay 1.0)
  (bind _asbp_player (Utilities|Casting|CastToBP_Player _returnvalue_2))
  (Variables|/Game/BP_Player.BP_Player_C|SetClientCamera _asbp_player self)
  (Variables|Default|SetPawnToFollow _returnvalue_2)
  (Game|Player|SetViewTargetwithBlend _returnvalue self 0.0 "VTBlend_Linear" 0.0 false)
  (Utilities|Time|SetTimerbyFunctionName 0 "UpdateCamera" 0.001 true))

(fn ConstructionScript)