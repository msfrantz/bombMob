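; Networked Bomberman-style bomb that explodes on a timer or on contact with another explosion, refunding its creator's bomb count after a delay.
; Freezing pauses the fuse and pulsing timeline while showing a custom-depth effect.
; Unless in water, detonation line-traces four grid directions per step, spawning BP_Explosion where clear and destroying destructible tiles.
; Collision switches to the Bombs profile when a player steps off; multicasts handle sound and hiding.
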(event OnComponentEndOverlap(Box)
  (params (OverlappedComponent :type Primitive%20Component%20Object%20Reference) (OtherActor :type Actor%20Object%20Reference) (OtherComp :type Primitive%20Component%20Object%20Reference) (OtherBodyIndex :type Integer))
  (Utilities|IsValid OtherActor
    (:Is%20Valid
      (if (Actor|ActorHasTag OtherActor "Player")
        (if (not (Variables|Default|GethasExploded))
          (Collision|SetCollisionProfileName (Variables|Collision|GetBox) "Bombs" :!class /Script/Engine.PrimitiveComponent))))))

(event OnComponentBeginOverlap(Box)
  (params (OverlappedComponent :type Primitive%20Component%20Object%20Reference) (OtherActor :type Actor%20Object%20Reference) (OtherComp :type Primitive%20Component%20Object%20Reference) (OtherBodyIndex :type Integer) (bFromSweep :type Boolean) (SweepResult :type Hit%20Result%20Structure%20%28by%20ref%29))
  (Utilities|IsValid OtherActor
    (:Is%20Valid
      (if (Actor|ActorHasTag OtherActor "Explosion")
        (Utilities|FlowControl|DoOnce false
          (:Completed
            (CallFunction|ServerSpawnExplosions)))))))

(event Custom|ServerSpawnExplosions
  (bind _returnvalue (Transformation|GetActorTransform))
  (bind _returnvalue_2 (Transformation|GetActorTransform))
  (bind _returnvalue_3 (Transformation|GetActorTransform))
  (bind _returnvalue_4 (Transformation|GetActorTransform))
  (bind _box (Variables|Collision|GetBox))
  ;[1 1 1] Explosion Spawn Loop
  (Variables|Default|SethasExploded true)
  (Collision|SetCollisionResponsetoAllChannels _box "ECR_Ignore")
  (Collision|SetCollisionProfileName _box "NoCollision" :!class /Script/Engine.PrimitiveComponent)
  (if (not (Variables|Default|GetfallenIntoWater))
    (CallFunction|MulticastExplosionSound)
    (Game|SpawnActorfromClass "/Game/BP_Explosion.BP_Explosion_C" (Transformation|GetActorTransform) "Undefined" 0 0)
    (for _index (range 1 (Variables|Default|GetExplosionLength))
      ;[1 1 1] Check for Walls and obstacles
      (bind (_outhit _returnvalue_5) (Collision|LineTraceForObjects (Math|Vector|MakeVector (.x (.location _returnvalue)) (.y (.location _returnvalue)) 1e+02) (Math|Vector|MakeVector (.x (.location _returnvalue)) (+ (.y (.location _returnvalue)) (Math|Conversions|ToFloat(Integer) (* _index 100))) 1e+02) (Variables|Default|GetObjectsToFind) false 0 "None"))
      (if _returnvalue_5
        (if (Actor|ActorHasTag (.HitActor (Collision|BreakHitResult _outhit)) "Destructible")
          (bind _asdestructible_tile (Utilities|Casting|CastToDestructibleTile (.HitActor (Collision|BreakHitResult _outhit))))
          (Default|DestroyObject _asdestructible_tile))
        (else
          (bind _returnvalue_6 (Game|SpawnActorfromClass "/Game/BP_Explosion.BP_Explosion_C" (Math|Transform|MakeTransform (Math|Vector|MakeVector (.x (.location _returnvalue)) (+ (.y (.location _returnvalue)) (Math|Conversions|ToFloat(Integer) (* _index 100))) (.z (.location _returnvalue))) (.rotation _returnvalue) (.scale _returnvalue)) "AlwaysSpawn" 0 0))
          (Variables|/Game/BP_Explosion.BP_Explosion_C|SetCreator _returnvalue_6 (Variables|Default|GetCreator))))
      (bind (_outhit_2 _returnvalue_7) (Collision|LineTraceForObjects (Math|Vector|MakeVector (.x (.location _returnvalue_2)) (.y (.location _returnvalue_2)) 1e+02) (Math|Vector|MakeVector (.x (.location _returnvalue_2)) (+ (Math|Conversions|ToFloat(Integer) (* _index -100)) (.y (.location _returnvalue_2))) 1e+02) (Variables|Default|GetObjectsToFind) false 0 "None"))
      (if _returnvalue_7
        (if (Actor|ActorHasTag (.HitActor (Collision|BreakHitResult _outhit_2)) "Destructible")
          (bind _asdestructible_tile_2 (Utilities|Casting|CastToDestructibleTile (.HitActor (Collision|BreakHitResult _outhit_2))))
          (Default|DestroyObject _asdestructible_tile_2))
        (else
          (bind _returnvalue_8 (Game|SpawnActorfromClass "/Game/BP_Explosion.BP_Explosion_C" (Math|Transform|MakeTransform (Math|Vector|MakeVector (.x (.location _returnvalue_2)) (+ (Math|Conversions|ToFloat(Integer) (* _index -100)) (.y (.location _returnvalue_2))) (.z (.location _returnvalue_2))) (.rotation _returnvalue_2) (.scale _returnvalue_2)) "AlwaysSpawn" 0 0))
          (Variables|/Game/BP_Explosion.BP_Explosion_C|SetCreator _returnvalue_8 (Variables|Default|GetCreator))))
      (bind (_outhit_3 _returnvalue_9) (Collision|LineTraceForObjects (Math|Vector|MakeVector (.x (.location _returnvalue_3)) (.y (.location _returnvalue_3)) 1e+02) (Math|Vector|MakeVector (+ (Math|Conversions|ToFloat(Integer) (* _index 100)) (.x (.location _returnvalue_3))) (.y (.location _returnvalue_3)) 1e+02) (Variables|Default|GetObjectsToFind) false 0 "None"))
      (if _returnvalue_9
        (if (Actor|ActorHasTag (.HitActor (Collision|BreakHitResult _outhit_3)) "Destructible")
          (bind _asdestructible_tile_3 (Utilities|Casting|CastToDestructibleTile (.HitActor (Collision|BreakHitResult _outhit_3))))
          (Default|DestroyObject _asdestructible_tile_3))
        (else
          (bind _returnvalue_10 (Game|SpawnActorfromClass "/Game/BP_Explosion.BP_Explosion_C" (Math|Transform|MakeTransform (Math|Vector|MakeVector (+ (Math|Conversions|ToFloat(Integer) (* _index 100)) (.x (.location _returnvalue_3))) (.y (.location _returnvalue_3)) (.z (.location _returnvalue_3))) (.rotation _returnvalue_3) (.scale _returnvalue_3)) "AlwaysSpawn" 0 0))
          (Variables|/Game/BP_Explosion.BP_Explosion_C|SetCreator _returnvalue_10 (Variables|Default|GetCreator))))
      (bind (_outhit_4 _returnvalue_11) (Collision|LineTraceForObjects (Math|Vector|MakeVector (.x (.location _returnvalue_4)) (.y (.location _returnvalue_4)) 1e+02) (Math|Vector|MakeVector (+ (Math|Conversions|ToFloat(Integer) (* _index -100)) (.x (.location _returnvalue_4))) (.y (.location _returnvalue_4)) 1e+02) (Variables|Default|GetObjectsToFind) false 0 "None"))
      (if _returnvalue_11
        (if (Actor|ActorHasTag (.HitActor (Collision|BreakHitResult _outhit_4)) "Destructible")
          (bind _asdestructible_tile_4 (Utilities|Casting|CastToDestructibleTile (.HitActor (Collision|BreakHitResult _outhit_4))))
          (Default|DestroyObject _asdestructible_tile_4))
        (else
          (bind _returnvalue_12 (Game|SpawnActorfromClass "/Game/BP_Explosion.BP_Explosion_C" (Math|Transform|MakeTransform (Math|Vector|MakeVector (+ (Math|Conversions|ToFloat(Integer) (* _index -100)) (.x (.location _returnvalue_4))) (.y (.location _returnvalue_4)) (.z (.location _returnvalue_4))) (.rotation _returnvalue_4) (.scale _returnvalue_4)) "AlwaysSpawn" 0 0))
          (Variables|/Game/BP_Explosion.BP_Explosion_C|SetCreator _returnvalue_12 (Variables|Default|GetCreator))))))
  (CallFunction|MulticastHideBomb)
  (Utilities|FlowControl|Delay 8.0)
  (Actor|DestroyActor))

(event Custom|BombExplode
  (Utilities|FlowControl|DoOnce false
    (:Completed
      (CallFunction|ServerSpawnExplosions))))

(event Custom|MulticastHideBomb
  (Collision|SetCollisionEnabled (Variables|Collision|GetBox) "NoCollision")
  (Collision|SetCollisionProfileName (Variables|Collision|GetBox) "NoCollision" :!class /Script/Engine.PrimitiveComponent)
  (Collision|SetCollisionObjectType (Variables|Collision|GetBox) "ECC_WorldStatic")
  (Rendering|SetVisibility (Variables|Default|GetDefaultSceneRoot) false true))

(event Custom|ServerFreezeBomb
  (params (Delay :type Float%20%28single-precision%29))
  (CallFunction|MulticastFreezeBomb Delay)
  (Class|KismetSystemLibrary|PauseTimer 0 "BombExplode")
  (Utilities|FlowControl|Delay Delay)
  (Class|KismetSystemLibrary|UnPauseTimer 0 "BombExplode"))

(event Custom|MulticastFreezeBomb
  (params (Delay :type Float%20%28single-precision%29))
  (bind _mesh (Variables|Default|Getmesh))
  (Utilities|FlowControl|Sequence
    (:then_0
      (Rendering|SetRenderCustomDepth (Variables|Default|Getmesh) true)
      (Utilities|FlowControl|Delay Delay)
      (Rendering|SetRenderCustomDepth (Variables|Default|Getmesh) false)
      (bind (_direction _scale _firepos _color) (Timeline|Timeline_0 Play)
        (:Update
          (Transformation|SetRelativeScale3D _mesh _scale)
          (bind _returnvalue (Rendering|Material|CreateDynamicMaterialInstance _mesh 0 "/Game/Art/BombMat.BombMat" "None" :!class /Script/Engine.PrimitiveComponent))
          (Rendering|Material|SetVectorParameterValue _returnvalue "Emissive Color" _color :!class /Script/Engine.MaterialInstanceDynamic)
          (Transformation|SetRelativeLocation (Variables|Default|GetFire) _firepos false false))))
    (:then_1
      (Timeline|Timeline_0 Stop))))

(event Custom|MulticastExplosionSound
  (Audio|PlaySoundatLocation "/Game/Sound/BombMobExplosion.BombMobExplosion" (Transformation|GetActorLocation) "0, 0, 0" 1.3 1.0 0.0 0 0 0))

(event EventBeginPlay
  (bind _mesh (Variables|Default|Getmesh))
  (bind _creator (Variables|Default|GetCreator))
  (Utilities|FlowControl|Sequence
    (:then_0
      (bind (_direction _scale _firepos _color) (Timeline|Timeline_0 PlayFromStart)
        (:Update
          (Transformation|SetRelativeScale3D _mesh _scale)
          (bind _returnvalue (Rendering|Material|CreateDynamicMaterialInstance _mesh 0 "/Game/Art/BombMat.BombMat" "None" :!class /Script/Engine.PrimitiveComponent))
          (Rendering|Material|SetVectorParameterValue _returnvalue "Emissive Color" _color :!class /Script/Engine.MaterialInstanceDynamic)
          (Transformation|SetRelativeLocation (Variables|Default|GetFire) _firepos false false))))
    (:then_1
      (Utilities|Time|SetTimerbyFunctionName 0 "BombExplode" 3.0))
    (:then_2
      (Utilities|FlowControl|Delay 5.0)
      (Utilities|IsValid _creator
        (:Is%20Valid
          (Math|Integer|IncrementInt (Variables|/Game/BP_Player.BP_Player_C|GetBombs _creator)))))))

(fn ConstructionScript)