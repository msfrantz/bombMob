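; BP_IceSpell is a short-lived area spell actor that freezes players and bombs.
; On BeginPlay it spawns an attached Niagara ice effect, briefly enables its box collision after a wind-up delay, then destroys itself shortly afterward.
; Overlaps are sorted by the actor's first tag, calling server freeze events on bombs and on players whose team differs from the spell's.
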(event OnComponentBeginOverlap(Box)
  (params (OverlappedComponent :type Primitive%20Component%20Object%20Reference) (OtherActor :type Actor%20Object%20Reference) (OtherComp :type Primitive%20Component%20Object%20Reference) (OtherBodyIndex :type Integer) (bFromSweep :type Boolean) (SweepResult :type Hit%20Result%20Structure%20%28by%20ref%29))
  (switch string (Utilities|String|ToString(Name) (Utilities|Array|Get(acopy) (Variables|/Script/Engine.Actor|GetTags OtherActor)))
    (:Player
      (bind _asbp_player (Utilities|Casting|CastToBP_Player OtherActor))
      (if (not (Utilities|Enum|Equal(Enum) (.MyPlayerTeam (Utilities|Struct|BreakPlayerInfo (Variables|/Game/BP_Player.BP_Player_C|GetPlayerInformation _asbp_player))) (Variables|Default|GetTeam)))
        (Default|ServerFreezePlayer _asbp_player 2.0)))
    (:Bomb
      (bind _asbp_bomb (Utilities|Casting|CastToBP_Bomb OtherActor))
      (Default|ServerFreezeBomb _asbp_bomb 2.0))))

(event Custom|ClientSpawnSpell
  (Niagara|SpawnSystemAttached "/Game/Art/Ice_Spell.Ice_Spell" (Variables|Default|GetBox) "None" "0, 0, 0" "0, 0, 0" "KeepRelativeOffset" true))

(event EventBeginPlay
  (Utilities|FlowControl|Sequence
    (:then_0
      (Utilities|FlowControl|Delay 3.0)
      (Actor|DestroyActor))
    (:then_1
      (Utilities|FlowControl|Delay 1.5)
      (Collision|SetCollisionEnabled (Variables|Default|GetBox) "QueryAndPhysics")
      (Utilities|FlowControl|Delay 0.3)
      (Collision|SetCollisionEnabled (Variables|Default|GetBox) "NoCollision"))
    (:then_2
      (CallFunction|ClientSpawnSpell))))

(event EventTick
  (params (DeltaSeconds :type Float%20%28single-precision%29)))

(fn ConstructionScript)