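; BP_Smoke is a short-lived smoke effect actor that plays a smoke explosion and its sound where it spawns.
; On BeginPlay it spawns a Niagara-style smoke system at its location and plays the smoke bomb sound through a multicast-named event.
; It destroys itself after a fixed delay, and Tick is unused.
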(event Custom|MulticastSound
  (Audio|PlaySoundatLocation "/Game/Sound/BombMobNinjaSmoke.BombMobNinjaSmoke" (Transformation|GetActorLocation) "0, 0, 0" 1.0 1.0 0.0 0 0 0))

(event Custom|ClientSpawnExplosion
  (Niagara|SpawnSystematLocation "/Game/Art/Smoke_Explosion2.Smoke_Explosion2" (Transformation|GetActorLocation)))

(event EventBeginPlay
  (Utilities|FlowControl|Sequence
    (:then_0
      (Utilities|FlowControl|Delay 1e+01)
      (Actor|DestroyActor))
    (:then_1
      (CallFunction|ClientSpawnExplosion)
      (CallFunction|MulticastSound))))

(event EventTick
  (params (DeltaSeconds :type Float%20%28single-precision%29)))

(fn ConstructionScript)